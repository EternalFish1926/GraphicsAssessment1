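; BP_Piano is an interactable piano puzzle actor that reveals the pantry key once solved.
; Overlap adds an outline overlay and, for the first-person character, enables input so IA_Interact opens WBP_Piano with a reference back to the piano.
; CompletePuzzle disables input, unhides the key, hides the piano, shows a solved message for three seconds, then destroys the actor.
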(event `EnhancedInput|/Game/Input/Actions/IA_Interact`
  (params (ActionValue :type Boolean) (ElapsedSeconds :type "Float (double-precision)") (TriggeredSeconds :type "Float (double-precision)") (InputAction :type "InputAction Object Reference" :default "/Game/Input/Actions/IA_Interact.IA_Interact"))
  (:`Started`
    (if (`self.PlayerInRange`)
      (bind _returnvalue (`|CreateWidget` "/Game/Input/WBP_Piano.WBP_Piano_C" (`GameplayStatics.GetPlayerController` 0) self))
      (bind _output_get (set `self.PianoWidgetRef` _returnvalue))
      (`UserWidget.AddToViewport` _output_get 0)
      (`WidgetBlueprintLibrary.SetInputMode_GameAndUIEx` (`GameplayStatics.GetPlayerController` 0) null "DoNotLock" false))))

(event `self.ReceiveActorBeginOverlap`
  (params (OtherActor :type "Actor Object Reference"))
  (`MeshComponent.SetOverlayMaterial` (`self.Cube`) "/Game/Input/M_InteractOutline.M_InteractOutline" false 0)
  (cast `/Game/FirstPerson/Blueprints/BP_FirstPersonCharacter` OtherActor)
  (set `self.PlayerInRange` true)
  (`self.EnableInput` (`GameplayStatics.GetPlayerController` 0)))

(event `self.ReceiveActorEndOverlap`
  (params (OtherActor :type "Actor Object Reference"))
  (`MeshComponent.SetOverlayMaterial` (`self.Cube`) null false 0)
  (cast `/Game/FirstPerson/Blueprints/BP_FirstPersonCharacter` OtherActor)
  (set `self.PlayerInRange` false)
  (`self.DisableInput` (`GameplayStatics.GetPlayerController` 0)))

(event `CompletePuzzle`
  (if (not (`self.PuzzleCompleted`))
    (`self.DisableInput` (`GameplayStatics.GetPlayerController` 0))
    (set `self.PlayerInRange` false)
    (`self.SetActorHiddenInGame` (`self.PantryKeyRef`) false)
    (bind _returnvalue (`|CreateWidget` "/Game/Input/Text.Text_C"))
    (`UserWidget.AddToViewport` _returnvalue 0)
    (`/Game/Input/Text.ShowMessage` _returnvalue "Piano Puzzle: Solved" null null)
    (`self.SetActorHiddenInGame` true)
    (`KismetSystemLibrary.Delay` 3.0)
    (`Widget.RemoveFromParent` _returnvalue)
    (`self.K2_DestroyActor`)))

(fn `UserConstructionScript`)