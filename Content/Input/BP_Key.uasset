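; Front door key pickup that sets HasKey on BP_FirstPersonCharacter when the player presses Interact in range.
; Actor overlap toggles an outline overlay material on the key mesh for any actor, but only the player character sets the range flag and toggles input.
; On pickup it shows a Text widget message, hides itself, then removes the widget and destroys itself after a short delay.
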(event `EnhancedInput|/Game/Input/Actions/IA_Interact`
  (params (ActionValue :type Boolean) (ElapsedSeconds :type "Float (double-precision)") (TriggeredSeconds :type "Float (double-precision)") (InputAction :type "InputAction Object Reference" :default "/Game/Input/Actions/IA_Interact.IA_Interact"))
  (:`Started`
    (if (`self.PlayerInRange`)
      (bind _output_get (set `/Game/FirstPerson/Blueprints/BP_FirstPersonCharacter.HasKey` true (stale `self.ReceiveActorBeginOverlap` _asbp_first_person_character)))
      (if _output_get
        (bind _returnvalue (`|CreateWidget` "/Game/Input/Text.Text_C"))
        (`UserWidget.AddToViewport` _returnvalue 0)
        (`/Game/Input/Text.ShowMessage` _returnvalue "Picked up: Front Door Key" null null)
        (`self.SetActorHiddenInGame` true)
        (`KismetSystemLibrary.Delay` 3.0)
        (`Widget.RemoveFromParent` _returnvalue)
        (`self.K2_DestroyActor`)))))

(event `self.ReceiveActorBeginOverlap`
  (params (OtherActor :type "Actor Object Reference"))
  (`MeshComponent.SetOverlayMaterial` (`self.KeyMesh`) "/Game/Input/M_InteractOutline.M_InteractOutline" false 0)
  (bind _asbp_first_person_character (cast `/Game/FirstPerson/Blueprints/BP_FirstPersonCharacter` OtherActor))
  (set `self.PlayerInRange` true)
  (`self.EnableInput` (`GameplayStatics.GetPlayerController` 0)))

(event `self.ReceiveActorEndOverlap`
  (params (OtherActor :type "Actor Object Reference"))
  (`MeshComponent.SetOverlayMaterial` (`self.KeyMesh`) null false 0)
  (cast `/Game/FirstPerson/Blueprints/BP_FirstPersonCharacter` OtherActor)
  (set `self.PlayerInRange` false)
  (`self.DisableInput` (`GameplayStatics.GetPlayerController` 0)))

(fn `UserConstructionScript`)